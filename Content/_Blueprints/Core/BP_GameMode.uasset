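; Game mode that scatters randomized loot across the map on BeginPlay.
; It first totals the weights in the count, item type and per-type ID probability DataTables.
; For each DT_ItemGroupLocations row it spawns a BP_ItemGroup, gets random transforms from it, and makes weighted rolls for item count, distinct types (re-rolling duplicates) and IDs.
; Each result spawns the matching BP_WorldItem subclass, initialized with its ID.
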(event `self.ReceiveBeginPlay`
  (`self.GenerateItems`))

(fn `GenerateItems`
  (locals (ItemTypeArr :type "Array of /Game/_Blueprints/Datas/Enum/Item/E_ItemType Enum") (SpawnItemArr :type "Array of /Game/_Blueprints/Datas/Struct/ItemGeneration/ST_SpawnItem Structure") (SpawnTransforms :type "Array of Transform Structure") (ItemGroupRef :type "/Game/_Blueprints/Items/BP_ItemGroup Object Reference") (ItemType :type "/Game/_Blueprints/Datas/Enum/Item/E_ItemType Enum") (SpawnId :type Name) (NumberProbabilityInfo :type "/Game/_Blueprints/Datas/Struct/ItemGeneration/ST_ProbabilityInfo Structure") (SumPercent :type Integer) (ItemTypeProbabilityInfo :type "/Game/_Blueprints/Datas/Struct/ItemGeneration/ST_ProbabilityInfo Structure") (ItemIDProbabilityInfos :type "Map of /Game/_Blueprints/Datas/Enum/Item/E_ItemType Enum to /Game/_Blueprints/Datas/Struct/ItemGeneration/ST_ProbabilityInfo Structure"))
  ; 아이템에 대한 데이터테이블 가져오기
  (`|ExecutionSequence`
    (:`then_0`
      (set `local.SumPercent` 0)
      (bind _outrownames (`DataTableFunctionLibrary.GetDataTableRowNames` "/Game/_Blueprints/Datas/DataTable/ItemGeneration/DT_NumberProbabilitys.DT_NumberProbabilitys"))
      (for _array_element _outrownames
        (bind _returnvalue (`|GetDataTableRow` "/Game/_Blueprints/Datas/DataTable/ItemGeneration/DT_NumberProbabilitys.DT_NumberProbabilitys" _array_element)
          (:`then`
            (set `local.SumPercent` (+ (`local.SumPercent`) (break `/Game/_Blueprints/Datas/Struct/ItemGeneration/ST_NumberProbability` _returnvalue))))))
      (set `local.NumberProbabilityInfo` (make `/Game/_Blueprints/Datas/Struct/ItemGeneration/ST_ProbabilityInfo` (`local.SumPercent`) _outrownames)))
    (:`then_1`
      (set `local.SumPercent` 0)
      (bind _outrownames_2 (`DataTableFunctionLibrary.GetDataTableRowNames` "/Game/_Blueprints/Datas/DataTable/ItemGeneration/DT_ItemTypeProbability.DT_ItemTypeProbability"))
      (for _array_element_2 _outrownames_2
        (bind _returnvalue_2 (`|GetDataTableRow` "/Game/_Blueprints/Datas/DataTable/ItemGeneration/DT_ItemTypeProbability.DT_ItemTypeProbability" _array_element_2)
          (:`then`
            (set `local.SumPercent` (+ (`local.SumPercent`) (break `/Game/_Blueprints/Datas/Struct/ItemGeneration/ST_ItemTypeProbability` _returnvalue_2))))))
      (set `local.ItemTypeProbabilityInfo` (make `/Game/_Blueprints/Datas/Struct/ItemGeneration/ST_ProbabilityInfo` (`local.SumPercent`) _outrownames_2)))
    (:`then_2`
      (set `local.SumPercent` 0)
      (bind _outrownames_3 (`DataTableFunctionLibrary.GetDataTableRowNames` "/Game/_Blueprints/Datas/DataTable/ItemGeneration/DT_AmmoProbability.DT_AmmoProbability"))
      (for _array_element_3 _outrownames_3
        (bind _returnvalue_3 (`|GetDataTableRow` "/Game/_Blueprints/Datas/DataTable/ItemGeneration/DT_AmmoProbability.DT_AmmoProbability" _array_element_3)
          (:`then`
            (set `local.SumPercent` (+ (`local.SumPercent`) (break `/Game/_Blueprints/Datas/Struct/ItemGeneration/ST_ItemProbability` _returnvalue_3))))))
      (`BlueprintMapLibrary.Map_Add` (`local.ItemIDProbabilityInfos`) "NewEnumerator2" (make `/Game/_Blueprints/Datas/Struct/ItemGeneration/ST_ProbabilityInfo` (`local.SumPercent`) _outrownames_3)))
    (:`then_3`
      (set `local.SumPercent` 0)
      (bind _outrownames_4 (`DataTableFunctionLibrary.GetDataTableRowNames` "/Game/_Blueprints/Datas/DataTable/ItemGeneration/DT_HealthProbability.DT_HealthProbability"))
      (for _array_element_4 _outrownames_4
        (bind _returnvalue_4 (`|GetDataTableRow` "/Game/_Blueprints/Datas/DataTable/ItemGeneration/DT_HealthProbability.DT_HealthProbability" _array_element_4)
          (:`then`
            (set `local.SumPercent` (+ (`local.SumPercent`) (break `/Game/_Blueprints/Datas/Struct/ItemGeneration/ST_ItemProbability` _returnvalue_4))))))
      (`BlueprintMapLibrary.Map_Add` (`local.ItemIDProbabilityInfos`) "NewEnumerator3" (make `/Game/_Blueprints/Datas/Struct/ItemGeneration/ST_ProbabilityInfo` (`local.SumPercent`) _outrownames_4)))
    (:`then_4`
      (set `local.SumPercent` 0)
      (bind _outrownames_5 (`DataTableFunctionLibrary.GetDataTableRowNames` "/Game/_Blueprints/Datas/DataTable/ItemGeneration/DT_BoostProbability.DT_BoostProbability"))
      (for _array_element_5 _outrownames_5
        (bind _returnvalue_5 (`|GetDataTableRow` "/Game/_Blueprints/Datas/DataTable/ItemGeneration/DT_BoostProbability.DT_BoostProbability" _array_element_5)
          (:`then`
            (set `local.SumPercent` (+ (`local.SumPercent`) (break `/Game/_Blueprints/Datas/Struct/ItemGeneration/ST_ItemProbability` _returnvalue_5))))))
      (`BlueprintMapLibrary.Map_Add` (`local.ItemIDProbabilityInfos`) "NewEnumerator4" (make `/Game/_Blueprints/Datas/Struct/ItemGeneration/ST_ProbabilityInfo` (`local.SumPercent`) _outrownames_5)))
    (:`then_5`
      (set `local.SumPercent` 0)
      (bind _outrownames_6 (`DataTableFunctionLibrary.GetDataTableRowNames` "/Game/_Blueprints/Datas/DataTable/ItemGeneration/DT_HelmetProbability.DT_HelmetProbability"))
      (for _array_element_6 _outrownames_6
        (bind _returnvalue_6 (`|GetDataTableRow` "/Game/_Blueprints/Datas/DataTable/ItemGeneration/DT_HelmetProbability.DT_HelmetProbability" _array_element_6)
          (:`then`
            (set `local.SumPercent` (+ (`local.SumPercent`) (break `/Game/_Blueprints/Datas/Struct/ItemGeneration/ST_ItemProbability` _returnvalue_6))))))
      (`BlueprintMapLibrary.Map_Add` (`local.ItemIDProbabilityInfos`) "NewEnumerator5" (make `/Game/_Blueprints/Datas/Struct/ItemGeneration/ST_ProbabilityInfo` (`local.SumPercent`) _outrownames_6)))
    (:`then_6`
      (set `local.SumPercent` 0)
      (bind _outrownames_7 (`DataTableFunctionLibrary.GetDataTableRowNames` "/Game/_Blueprints/Datas/DataTable/ItemGeneration/DT_VestProbability.DT_VestProbability"))
      (for _array_element_7 _outrownames_7
        (bind _returnvalue_7 (`|GetDataTableRow` "/Game/_Blueprints/Datas/DataTable/ItemGeneration/DT_VestProbability.DT_VestProbability" _array_element_7)
          (:`then`
            (set `local.SumPercent` (+ (`local.SumPercent`) (break `/Game/_Blueprints/Datas/Struct/ItemGeneration/ST_ItemProbability` _returnvalue_7))))))
      (`BlueprintMapLibrary.Map_Add` (`local.ItemIDProbabilityInfos`) "NewEnumerator6" (make `/Game/_Blueprints/Datas/Struct/ItemGeneration/ST_ProbabilityInfo` (`local.SumPercent`) _outrownames_7)))
    (:`then_7`
      (set `local.SumPercent` 0)
      (bind _outrownames_8 (`DataTableFunctionLibrary.GetDataTableRowNames` "/Game/_Blueprints/Datas/DataTable/ItemGeneration/DT_BackpackProbability.DT_BackpackProbability"))
      (for _array_element_8 _outrownames_8
        (bind _returnvalue_8 (`|GetDataTableRow` "/Game/_Blueprints/Datas/DataTable/ItemGeneration/DT_BackpackProbability.DT_BackpackProbability" _array_element_8)
          (:`then`
            (set `local.SumPercent` (+ (`local.SumPercent`) (break `/Game/_Blueprints/Datas/Struct/ItemGeneration/ST_ItemProbability` _returnvalue_8))))))
      (`BlueprintMapLibrary.Map_Add` (`local.ItemIDProbabilityInfos`) "NewEnumerator7" (make `/Game/_Blueprints/Datas/Struct/ItemGeneration/ST_ProbabilityInfo` (`local.SumPercent`) _outrownames_8)))
    (:`then_8`
      (set `local.SumPercent` 0)
      (bind _outrownames_9 (`DataTableFunctionLibrary.GetDataTableRowNames` "/Game/_Blueprints/Datas/DataTable/ItemGeneration/DT_WeaponProbability.DT_WeaponProbability"))
      (for _array_element_9 _outrownames_9
        (bind _returnvalue_9 (`|GetDataTableRow` "/Game/_Blueprints/Datas/DataTable/ItemGeneration/DT_WeaponProbability.DT_WeaponProbability" _array_element_9)
          (:`then`
            (set `local.SumPercent` (+ (`local.SumPercent`) (break `/Game/_Blueprints/Datas/Struct/ItemGeneration/ST_ItemProbability` _returnvalue_9))))))
      (`BlueprintMapLibrary.Map_Add` (`local.ItemIDProbabilityInfos`) "NewEnumerator0" (make `/Game/_Blueprints/Datas/Struct/ItemGeneration/ST_ProbabilityInfo` (`local.SumPercent`) _outrownames_9)))
    (:`then_9`
      (set `local.SumPercent` 0)
      (bind _outrownames_10 (`DataTableFunctionLibrary.GetDataTableRowNames` "/Game/_Blueprints/Datas/DataTable/ItemGeneration/DT_WeaponAccProbability.DT_WeaponAccProbability"))
      (for _array_element_10 _outrownames_10
        (bind _returnvalue_10 (`|GetDataTableRow` "/Game/_Blueprints/Datas/DataTable/ItemGeneration/DT_WeaponAccProbability.DT_WeaponAccProbability" _array_element_10)
          (:`then`
            (set `local.SumPercent` (+ (`local.SumPercent`) (break `/Game/_Blueprints/Datas/Struct/ItemGeneration/ST_ItemProbability` _returnvalue_10))))))
      (`BlueprintMapLibrary.Map_Add` (`local.ItemIDProbabilityInfos`) "NewEnumerator1" (make `/Game/_Blueprints/Datas/Struct/ItemGeneration/ST_ProbabilityInfo` (`local.SumPercent`) _outrownames_10)))
    (:`then_10`
      ; 위치를 지정한 아이템그룹들을 스폰
      ;; dataTable 의 전체 로우네임 가져오기
      (bind _outrownames_11 (`DataTableFunctionLibrary.GetDataTableRowNames` "/Game/_Blueprints/Datas/DataTable/ItemGeneration/DT_ItemGroupLocations.DT_ItemGroupLocations"))
      (for _array_element_11 _outrownames_11
        (bind _returnvalue_11 (`|GetDataTableRow` "/Game/_Blueprints/Datas/DataTable/ItemGeneration/DT_ItemGroupLocations.DT_ItemGroupLocations" _array_element_11)
          (:`then`
            (bind _returnvalue_12 (`|SpawnActorFromClass` "/Game/_Blueprints/Items/BP_ItemGroup.BP_ItemGroup_C" (`KismetMathLibrary.MakeTransform` (break `/Game/_Blueprints/Datas/Struct/ItemGeneration/ST_ItemGroupLocation` _returnvalue_11)) "Undefined" "MultiplyWithRoot" null null))
            (set `local.ItemGroupRef` _returnvalue_12)
            (`KismetArrayLibrary.Array_Clear` (`local.ItemTypeArr`))
            ; 아이템 그룹에 생성될 랜덤 아이템 개수 정하기
            (bind _number (`self.RandomItemNumber` (`local.NumberProbabilityInfo`)))
            (set `local.SpawnTransforms` (`/Game/_Blueprints/Items/BP_ItemGroup.GetRandomTreansforms` (`local.ItemGroupRef`) _number))
            (for _ (range 1 (+ _number 1))
              ; 랜덤한 아이템 타입 정하기
              (bind _itemtype (`self.RandomItemType` (`local.ItemTypeProbabilityInfo`) :!label _label))
              ; 랜덤한 아이템끼리 중복방지
              (if (== (`KismetArrayLibrary.Array_Find` (`local.ItemTypeArr`) _itemtype) -1)
                (`KismetArrayLibrary.Array_Add` (`local.ItemTypeArr`) _itemtype)
                (else
                  (goto _label))))
            (for _array_element_12 (`local.ItemTypeArr`)
              (bind _spawnitem (`self.RandomItemId` (`local.ItemIDProbabilityInfos`) _array_element_12))
              (`KismetArrayLibrary.Array_Add` (`local.SpawnItemArr`) _spawnitem))
            (for (_array_element_13 _array_index) (`local.SpawnItemArr`)
              (set `local.ItemType` (break `/Game/_Blueprints/Datas/Struct/ItemGeneration/ST_SpawnItem` _array_element_13))
              (set `local.SpawnId` (`.ID_5_2507E0114A0FD9AA074D76B63D71CED0` (break `/Game/_Blueprints/Datas/Struct/ItemGeneration/ST_SpawnItem` _array_element_13)))
              (bind _returnvalue_13 (`|SpawnActorFromClass` (select `/Game/_Blueprints/Datas/Enum/Item/E_ItemType` (`local.ItemType`) :`NewEnumerator0` "/Game/_Blueprints/Items/WorldItems/BP_WorldItem_Weapon.BP_WorldItem_Weapon_C" :`NewEnumerator1` "/Game/_Blueprints/Items/WorldItems/BP_WorldItem_WeaponAcc.BP_WorldItem_WeaponAcc_C" :`NewEnumerator2` "/Game/_Blueprints/Items/WorldItems/BP_WorldItem_Ammo.BP_WorldItem_Ammo_C" :`NewEnumerator3` "/Game/_Blueprints/Items/WorldItems/BP_WorldItem_Health.BP_WorldItem_Health_C" :`NewEnumerator4` "/Game/_Blueprints/Items/WorldItems/BP_WorldItem_Boost.BP_WorldItem_Boost_C" :`NewEnumerator5` "/Game/_Blueprints/Items/WorldItems/BP_WorldItem_Helmet.BP_WorldItem_Helmet_C" :`NewEnumerator6` "/Game/_Blueprints/Items/WorldItems/BP_WorldItem_Vest.BP_WorldItem_Vest_C" :`NewEnumerator7` "/Game/_Blueprints/Items/WorldItems/BP_WorldItem_Backpack.BP_WorldItem_Backpack_C" :!type "Actor Class Reference") (`|GetArrayItem` (`local.SpawnTransforms`) _array_index) "Undefined" "MultiplyWithRoot" null null))
              (bind _asbp_world_item_base (cast `/Game/_Blueprints/Items/WorldItems/BP_WorldItemBase` _returnvalue_13))
              (`/Game/_Blueprints/Items/WorldItems/BP_WorldItemBase.InitSpawnData` _asbp_world_item_base (`local.SpawnId`) "1"))
            (`KismetArrayLibrary.Array_Clear` (`local.SpawnItemArr`))))))))

(fn `RandomItemId`
  (params (ItemIDProbabilityInfo :type "Map of /Game/_Blueprints/Datas/Enum/Item/E_ItemType Enum to /Game/_Blueprints/Datas/Struct/ItemGeneration/ST_ProbabilityInfo Structure") (ItemType :type "/Game/_Blueprints/Datas/Enum/Item/E_ItemType Enum" :default "NewEnumerator0"))
  (returns (SpawnItem :type "/Game/_Blueprints/Datas/Struct/ItemGeneration/ST_SpawnItem Structure"))
  (locals (ItemArr :type "Array of /Game/_Blueprints/Datas/Struct/ItemGeneration/ST_SpawnItem Structure") (RandomValue :type Integer) (SumPercent :type Integer))
  (bind (_totalpercent _rownames) (break `/Game/_Blueprints/Datas/Struct/ItemGeneration/ST_ProbabilityInfo` (`BlueprintMapLibrary.Map_Find` ItemIDProbabilityInfo ItemType)))
  (set `local.RandomValue` (`KismetMathLibrary.RandomIntegerInRange` 1 _totalpercent))
  (for _array_element _rownames
    (bind _returnvalue (`|GetDataTableRow` (select `/Game/_Blueprints/Datas/Enum/Item/E_ItemType` (`local.ItemType`) :`NewEnumerator0` "/Game/_Blueprints/Datas/DataTable/ItemGeneration/DT_WeaponProbability.DT_WeaponProbability" :`NewEnumerator1` "/Game/_Blueprints/Datas/DataTable/ItemGeneration/DT_WeaponAccProbability.DT_WeaponAccProbability" :`NewEnumerator2` "/Game/_Blueprints/Datas/DataTable/ItemGeneration/DT_AmmoProbability.DT_AmmoProbability" :`NewEnumerator3` "/Game/_Blueprints/Datas/DataTable/ItemGeneration/DT_HealthProbability.DT_HealthProbability" :`NewEnumerator4` "/Game/_Blueprints/Datas/DataTable/ItemGeneration/DT_BoostProbability.DT_BoostProbability" :`NewEnumerator5` "/Game/_Blueprints/Datas/DataTable/ItemGeneration/DT_HelmetProbability.DT_HelmetProbability" :`NewEnumerator6` "/Game/_Blueprints/Datas/DataTable/ItemGeneration/DT_VestProbability.DT_VestProbability" :`NewEnumerator7` "/Game/_Blueprints/Datas/DataTable/ItemGeneration/DT_BackpackProbability.DT_BackpackProbability" :!type "DataTable Object Reference") _array_element)
      (:`then`
        (bind _output_get (set `local.SumPercent` (+ (`local.SumPercent`) (`.Percent_2_96E3891B42DDCA0F15A4A8B7E55CEB68` (break `/Game/_Blueprints/Datas/Struct/ItemGeneration/ST_ItemProbability` _returnvalue)))))
        (if (>= _output_get (`local.RandomValue`))
          (return (make `/Game/_Blueprints/Datas/Struct/ItemGeneration/ST_SpawnItem` (`local.ItemType`) _array_element)))))))

(fn `RandomItemNumber`
  (params (NumberProbability :type "/Game/_Blueprints/Datas/Struct/ItemGeneration/ST_ProbabilityInfo Structure"))
  (returns (Number :type Integer))
  (locals (NumberArr :type "Array of Integer") (SumPercent :type Integer) (RandomValue :type Integer))
  (set `local.RandomValue` (`KismetMathLibrary.RandomIntegerInRange` 1 NumberProbability_TotalPercent_2_2685E735442E8D4870EBF29958D01A59))
  ; 총 3회 순회
  (for _array_element NumberProbability_RowNames_6_054A0857498E2D07E1623CA6DB6D2DBF
    (bind _returnvalue (`|GetDataTableRow` "/Game/_Blueprints/Datas/DataTable/ItemGeneration/DT_NumberProbabilitys.DT_NumberProbabilitys" _array_element)
      (:`then`
        (bind _output_get (set `local.SumPercent` (+ (`local.SumPercent`) (break `/Game/_Blueprints/Datas/Struct/ItemGeneration/ST_NumberProbability` _returnvalue))))
        (if (>= _output_get (`local.RandomValue`))
          (return (`.Number_5_2D7BFD224C5A7E3ED404AABE27E666DB` (break `/Game/_Blueprints/Datas/Struct/ItemGeneration/ST_NumberProbability` _returnvalue))))))))

(fn `RandomItemType`
  (params (ItemTypeProbabilityInfo :type "/Game/_Blueprints/Datas/Struct/ItemGeneration/ST_ProbabilityInfo Structure"))
  (returns (ItemType :type "/Game/_Blueprints/Datas/Enum/Item/E_ItemType Enum"))
  (locals (ItemTypeArr :type "Array of /Game/_Blueprints/Datas/Enum/Item/E_ItemType Enum") (SumPercent :type Integer) (RandomValue :type Integer))
  (set `local.RandomValue` (`KismetMathLibrary.RandomIntegerInRange` 1 ItemTypeProbabilityInfo_TotalPercent_2_2685E735442E8D4870EBF29958D01A59))
  (for _array_element ItemTypeProbabilityInfo_RowNames_6_054A0857498E2D07E1623CA6DB6D2DBF
    (bind _returnvalue (`|GetDataTableRow` "/Game/_Blueprints/Datas/DataTable/ItemGeneration/DT_ItemTypeProbability.DT_ItemTypeProbability" _array_element)
      (:`then`
        (bind _output_get (set `local.SumPercent` (+ (`local.SumPercent`) (break `/Game/_Blueprints/Datas/Struct/ItemGeneration/ST_ItemTypeProbability` _returnvalue))))
        (if (>= _output_get (`local.RandomValue`))
          (return (`.ItemType_5_2E9D28F5442FECA94D9EA395D74AA29C` (break `/Game/_Blueprints/Datas/Struct/ItemGeneration/ST_ItemTypeProbability` _returnvalue))))))))

(fn `UserConstructionScript`)