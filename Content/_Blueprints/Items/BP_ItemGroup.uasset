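; BP_ItemGroup is an item-group actor that generates random positions around itself, presumably for placing a group's items.
; GetRandomTreansforms returns the requested number of world-space transforms, each offset from the actor's location on X and Y using random unit vectors scaled by a random distance.
; The Z offset is zero, with default rotation and scale.
; The event graph and construction script are empty, and nothing here spawns items.
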(fn `GetRandomTreansforms`
  (params (Number :type Integer))
  (returns (NewParam :type "Array of Transform Structure"))
  (locals (ReturnTransforms :type "Array of Transform Structure"))
  (bind (_returnvalue_x _returnvalue_y) (`KismetMathLibrary.BreakVector` (* (`KismetMathLibrary.RandomUnitVector`) (`KismetMathLibrary.RandomFloatInRange` 80.0 120.0))))
  ; 아이템 그룹 100~200CM이내 반경 랜덤한 위치 배열 생성
  (for _ (range 1 (+ Number 1))
    (`KismetArrayLibrary.Array_Add` (`local.ReturnTransforms`) (`KismetMathLibrary.MakeTransform` (+ (`self.K2_GetActorLocation`) (`KismetMathLibrary.MakeVector` _returnvalue_x _returnvalue_y)))))
  (return (`local.ReturnTransforms`)))

(fn `UserConstructionScript`)